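; Audio-reactive Niagara actor that morphs its particles to MetaSound output when the player is nearby.
; BeginPlay adds an audio component and watches a MetaSound amplitude-follower output through the MetaSound Output subsystem.
; Within a set distance of the player, that value drives the Niagara SoundMorph parameter, and after a short delay a timeline ramps ColorMorph.
; Out of range, the timeline stops; PlayerInRange is an empty stub.
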(event `self.ReceiveBeginPlay`
  ;[1 1 1] Binding to Any Message
  ;;[0.1651 0.7991 1] Play the MetaSound from the parent BluePrint
  (bind _returnvalue (`AddComponent|NODE_AddAudioComponent-0`))
  ;;[0.1651 0.7991 1] Receive MetaSound Output to control Niagara System Parameters
  (`MetaSoundOutputSubsystem.WatchOutput` (subsystem `MetaSoundOutputSubsystem`) _returnvalue "AmpFollowMonoTest" (delegate `AudioFloatOut`) "None" "None"))

(event `self.ReceiveTick`
  (params (DeltaSeconds :type "Float (single-precision)"))
  ;[1 1 1] Binding to Any Message
  ;;[1 1 1] Not Used But Could be in the future
)

(event `Player In Range`
  ;[1 1 1] Binding to Any Message
  ;;[1 1 1] Not Used But Could be in the future
)

(event `AudioFloatOut`
  (params (OutputName :type Name) (Output :type "MetaSoundOutput Structure (by ref)"))
  (bind _ns_deadend2 (`self.NS_DeadEnd2`))
  ;[1 1 1] Binding to Any Message
  ;;[0.1651 0.7991 1] Receive Audio From MetaSound to Control the 'Morph' Parameter of the Niagara System
  (bind (_success _returnvalue) (`MetasoundOutputBlueprintAccess.GetFloat` Output))
  (if (< (`self.GetDistanceTo` (`GameplayStatics.GetPlayerCharacter` 0) self) 650.0)
    (`FXSystemComponent.SetFloatParameter` _ns_deadend2 "User.SoundMorph" (* _returnvalue 5.0))
    (`KismetSystemLibrary.Delay` 0.5)
    (`self.Player In Range` self)
    ;;[0.1651 0.7991 1] Ramp The Color of the Niagara Particles Based on a Timeline
    (bind (_direction _fade) (`Timeline|Timeline_1` :!via `PlayFromStart` :!label _label)
      (:`Update`
        (`FXSystemComponent.SetFloatParameter` _ns_deadend2 "User.ColorMorph" _fade)
        (`self.Player In Range` self)))
    (else
      (goto _label :!via `Stop`))))

(fn `UserConstructionScript`)